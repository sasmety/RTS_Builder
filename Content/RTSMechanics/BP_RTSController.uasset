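; BP_RTSController is an RTS player controller that shows the mouse cursor and forwards left-click input to the HUD for marquee selection.
; Press and release of MouseLeftClick set a held flag and send marquee pressed and released messages to the HUD.
; While the flag is set, Tick sends a held message every frame, leaving the marquee logic itself to the HUD.
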(event `self.ReceiveBeginPlay`
  (set `self.bShowMouseCursor` true))

(event `self.ReceiveTick`
  (params (DeltaSeconds :type "Float (single-precision)"))
  (if (`self.bIsLeftClicked`)
    (message `/Game/RTSMechanics/BP_RTSInterface.MarqueeHeld` (`self.GetHUD`))))

(event `InputAction|MouseLeftClick`
  (params (Key :type "Key Structure"))
  (bind _returnvalue (`self.GetHUD`))
  (:`Pressed`
    (message `/Game/RTSMechanics/BP_RTSInterface.MarqueePressed` _returnvalue)
    (set `self.bIsLeftClicked` true))
  (:`Released`
    (message `/Game/RTSMechanics/BP_RTSInterface.MarqueeReleased` _returnvalue)
    (set `self.bIsLeftClicked` false)))

(fn `UserConstructionScript`)