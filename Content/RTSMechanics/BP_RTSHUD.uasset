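; RTS HUD that draws a marquee selection box and highlights the actors inside it.
; Press, hold and release events store the box corners as world points from a visibility trace, reprojected to screen each DrawHUD so the start stays world-anchored.
; While drawing, GetActorsInSelectionRectangle fills the selection and enables custom depth on static mesh components.
; Highlights clear only on the next press, for actors still in the last stored selection.
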(event `/Game/RTSMechanics/BP_RTSInterface.MarqueePressed`
  (bind _out_actors (`self.Out Actors`))
  (set `self.isDrawing?` true)
  (bind _out_hit_location (`self.LineTraceFromCursor`))
  (set `self.startVec` _out_hit_location)
  (set `self.currentVec` _out_hit_location)
  (for _array_element _out_actors
    (`PrimitiveComponent.SetRenderCustomDepth` (`self.K2_GetComponentsByClass` _array_element "/Script/Engine.StaticMeshComponent") false))
  (`KismetArrayLibrary.Array_Clear` _out_actors))

(event `/Game/RTSMechanics/BP_RTSInterface.MarqueeHeld`
  (bind _out_hit_location (`self.LineTraceFromCursor`))
  (set `self.currentVec` _out_hit_location))

(event `/Game/RTSMechanics/BP_RTSInterface.MarqueeReleased`
  (set `self.isDrawing?` false))

(event `self.ReceiveDrawHUD`
  (params (SizeX :type Integer) (SizeY :type Integer))
  (bind _returnvalue (`GameplayStatics.GetPlayerController` 0))
  (bind _screenposition (`GameplayStatics.ProjectWorldToScreen` _returnvalue (`self.startVec`)))
  (bind _screenposition_2 (`GameplayStatics.ProjectWorldToScreen` _returnvalue (`self.currentVec`)))
  (if (`self.isDrawing?`)
    (`self.DrawRect` (struct :`R` 0.163061 :`G` 0.227188 :`B` 0.807292 :`A` 0.656) (`KismetMathLibrary.BreakVector2D` _screenposition) (`.Y` (`KismetMathLibrary.BreakVector2D` _screenposition)) (- (`KismetMathLibrary.BreakVector2D` _screenposition_2) (`KismetMathLibrary.BreakVector2D` _screenposition)) (- (`.Y` (`KismetMathLibrary.BreakVector2D` _screenposition_2)) (`.Y` (`KismetMathLibrary.BreakVector2D` _screenposition))))
    (bind _output_get (set `self.Out Actors` (`self.GetActorsInSelectionRectangle` "/Script/Engine.Actor" (`KismetMathLibrary.MakeVector2D` (`KismetMathLibrary.BreakVector2D` _screenposition) (`.Y` (`KismetMathLibrary.BreakVector2D` _screenposition))) (`KismetMathLibrary.MakeVector2D` (`KismetMathLibrary.BreakVector2D` _screenposition_2) (`.Y` (`KismetMathLibrary.BreakVector2D` _screenposition_2))))))
    (for _array_element _output_get
      (`PrimitiveComponent.SetRenderCustomDepth` (`self.K2_GetComponentsByClass` _array_element "/Script/Engine.StaticMeshComponent") true))))

(fn `LineTraceFromCursor`
  (returns (`Out Hit Location` :type "Vector Structure"))
  (bind (_worldlocation _worlddirection) (`PlayerController.DeprojectMousePositionToWorld` (`GameplayStatics.GetPlayerController` 0)))
  (bind _outhit (`KismetSystemLibrary.LineTraceSingle` (0.0 0.0 0.0) (0.0 0.0 0.0) "TraceTypeQuery1"))
  (if true
    (return (`.Location` (`GameplayStatics.BreakHitResult` _outhit)))
    (else
      (return (+ _worldlocation (* _worlddirection 5000.0))))))

(fn `UserConstructionScript`)